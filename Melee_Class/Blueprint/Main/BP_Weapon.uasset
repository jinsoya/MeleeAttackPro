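; Melee weapon actor that works as a world pickup and runs the player's attacks once equipped.
; Sphere overlap shows a name/icon widget and custom-depth highlight, and interaction hands the weapon to WeaponEquipUnequip.
; Gates and timers play single or combo montages within timing windows, reading the equipped weapon's settings.
; A capsule overlap starts looping box traces that deal randomized damage through BP_Take_Damage or BP_Receive_Attack, spawn blood and reduce durability, which blocks attacks at zero.
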(event OnComponentBeginOverlap(Sphere)
  (params (OverlappedComponent :type Primitive%20Component%20Object%20Reference) (OtherActor :type Actor%20Object%20Reference) (OtherComp :type Primitive%20Component%20Object%20Reference) (OtherBodyIndex :type Integer) (bFromSweep :type Boolean) (SweepResult :type Hit%20Result%20Structure%20%28by%20ref%29))
  (bind _weaponsettings (Variables|Weapon|GetWeaponSettings))
  (bind _widgetweapon (Variables|Don'tchange|GetWidgetWeapon))
  (bind _widget (Variables|Default|GetWidget))
  (bind _skeletalmesh (Variables|Default|GetSkeletalMesh))
  (bind (_weapon_type _weapon_class _decrease_durability _current_state _damage _weapon_image) (Utilities|Struct|BreakS_Weapon_Settings _weaponsettings))
  ;[1 1 1] Sphere Collider
  (if (== OtherActor (Variables|Character|GetCharacter))
    (Rendering|Components|TextRender|SetText (Variables|/Game/MeleeSystemPro/Melee_Class/Widget/W_Weapon_Widget.W_Weapon_Widget_C|GetTextBlock_78 _widgetweapon) (Utilities|Text|ToText(String) (Utilities|String|EnumtoString _weapon_type)))
    (Appearance|SetBrushfromTexture (Variables|/Game/MeleeSystemPro/Melee_Class/Widget/W_Weapon_Widget.W_Weapon_Widget_C|GetImage_146 _widgetweapon) _weapon_image false)
    (UserInterface|SetWidget _widget _widgetweapon)
    (Transformation|SetWorldLocation _widget (+ (Transformation|GetWorldLocation (Variables|Default|GetSkeletalMesh)) "0, 0,70.000000") false false)
    (Rendering|SetVisibility _widget true false)
    (Rendering|SetRenderCustomDepth _skeletalmesh true)
    (Utilities|FlowControl|Delay 2.0)
    (Physics|SetSimulatePhysics _skeletalmesh false)))

(event OnComponentEndOverlap(Sphere)
  (params (OverlappedComponent :type Primitive%20Component%20Object%20Reference) (OtherActor :type Actor%20Object%20Reference) (OtherComp :type Primitive%20Component%20Object%20Reference) (OtherBodyIndex :type Integer))
  ;[1 1 1] Sphere Collider
  (if (== OtherActor (Variables|Character|GetCharacter))
    (Rendering|SetVisibility (Variables|Default|GetWidget) false false)
    (Rendering|SetRenderCustomDepth (Variables|Default|GetSkeletalMesh) false)))

(event OnComponentBeginOverlap(CapsuleHit)
  (params (OverlappedComponent :type Primitive%20Component%20Object%20Reference) (OtherActor :type Actor%20Object%20Reference) (OtherComp :type Primitive%20Component%20Object%20Reference) (OtherBodyIndex :type Integer) (bFromSweep :type Boolean) (SweepResult :type Hit%20Result%20Structure%20%28by%20ref%29))
  ;[1 1 1] Hit
  (bind _returnvalue (Utilities|Time|SetTimerbyEvent (delegate Custom|Attack) 0.01 true)))

(event Custom|OffAll
  ;[1 1 1] Destroy All
  (Rendering|SetVisibility (Variables|Default|GetWidget) false false)
  (Rendering|SetRenderCustomDepth (Variables|Default|GetSkeletalMesh) false)
  (Components|DestroyComponent (Variables|Default|GetSphere))
  (Collision|SetCollisionResponsetoChannel (Variables|Default|GetSkeletalMesh) "ECC_GameTraceChannel2" "ECR_Ignore"))

(event Custom|FirePress
  (params (WeaponEquipUnequip :type BP%20Melee%20Weapon%20Equip%20Unequip%20Object%20Reference))
  ;[1 1 1] Fire
  (bind _output_get (Variables|Default|SetWeaponEquipUnequip WeaponEquipUnequip))
  (Utilities|IsValid _output_get
    (:Is%20Valid
      (if (Variables|/Game/MeleeSystemPro/BP_MeleeWeapon_Equip_Unequip.BP_MeleeWeapon_Equip_Unequip_C|GetisSwap? _output_get)
        (CallFunction|StopFire :!label _label)
        (Variables|Don'tchange|SetisStop? true)
        (Utilities|FlowControl|Delay 0.2)
        (elif (Variables|/Game/MeleeSystemPro/BP_MeleeWeapon_Equip_Unequip.BP_MeleeWeapon_Equip_Unequip_C|GetisEquiped? _output_get)
          (if (<= (.Current_State (Utilities|Struct|BreakS_Weapon_Settings (Variables|BP_Weapon_C|GetWeaponSettings (Variables|/Game/MeleeSystemPro/BP_MeleeWeapon_Equip_Unequip.BP_MeleeWeapon_Equip_Unequip_C|GetCurrentWeapon (Variables|Default|GetWeaponEquipUnequip))))) 0)
            (goto _label)
            (else
              (Variables|Don'tchange|SetisStop? false)
              (Variables|Don'tchange|SetcanFire? true)
              (if (Utilities|Array|ContainsItem (Variables|/Game/MeleeSystemPro/BP_MeleeWeapon_Equip_Unequip.BP_MeleeWeapon_Equip_Unequip_C|GetEquipWeapon (Variables|Default|GetWeaponEquipUnequip)) true)
                (CallFunction|StartFire)
                (bind _returnvalue (Utilities|Time|SetTimerbyEvent (delegate Custom|Updating) 0.01 true)))))
          (else
            (goto _label)))))
    (:Is%20Not%20Valid
      (goto _label))))

(event Custom|EnableHit
  ;[1 1 1] Hit
  (Utilities|FlowControl|Delay 0.2)
  (Collision|SetCollisionEnabled (Variables|Default|GetCapsuleHit) "QueryAndPhysics"))

(event Custom|Attack
  (bind _character (Variables|Character|GetCharacter))
  (bind _weaponequipunequip (Variables|Default|GetWeaponEquipUnequip))
  (bind _capsulehit (Variables|Default|GetCapsuleHit))
  (bind _weaponequipunequip_2 (Variables|Default|GetWeaponEquipUnequip))
  (bind _returnvalue (Transformation|GetWorldLocation _capsulehit))
  (bind (_outradius _outhalfheight) (Class|CapsuleComponent|GetUnscaledCapsuleSize _capsulehit))
  (bind _currentweapon (Variables|/Game/MeleeSystemPro/BP_MeleeWeapon_Equip_Unequip.BP_MeleeWeapon_Equip_Unequip_C|GetCurrentWeapon _weaponequipunequip_2))
  (bind _currentweapon_2 (Variables|/Game/MeleeSystemPro/BP_MeleeWeapon_Equip_Unequip.BP_MeleeWeapon_Equip_Unequip_C|GetCurrentWeapon _weaponequipunequip))
  (bind _weaponsettings (Variables|BP_Weapon_C|GetWeaponSettings _currentweapon_2))
  (bind _weaponsettings_2 (Variables|BP_Weapon_C|GetWeaponSettings _currentweapon))
  (bind (_decrease_durability _current_state) (Utilities|Struct|BreakS_Weapon_Settings _weaponsettings))
  (bind _damage (Utilities|Struct|BreakS_Weapon_Settings _weaponsettings_2))
  (bind _returnvalue_2 (Math|Float|%(Float) _damage 2e+01))
  (bind _returnvalue_3 (- _damage _returnvalue_2))
  (bind _returnvalue_4 (Math|Random|RandomFloatinRange _returnvalue_3 _damage))
  ;[1 1 1] Hit
  (bind (_outhit _returnvalue_5) (Collision|BoxTraceByChannel _returnvalue _returnvalue (Math|Vector|MakeVector _outradius _outradius _outhalfheight) (Transformation|GetWorldRotation _capsulehit) "TraceTypeQuery1" false 0 "None"))
  (if _returnvalue_5
    (Utilities|Time|ClearandInvalidateTimerbyHandle (stale OnComponentBeginOverlap(CapsuleHit) _returnvalue))
    (if (Utilities|DoesObjectImplementInterface (.HitActor (Collision|BreakHitResult _outhit)) "/Game/MeleeSystemPro/Melee_Class/Blueprint/Interface/BP_Take_Damage.BP_Take_Damage_C")
      (Class|BPTakeDamage|ITakeDamage(Message) (.HitActor (Collision|BreakHitResult _outhit)) (.HitBoneName (Collision|BreakHitResult _outhit)) _returnvalue_4 _character (.Location (Collision|BreakHitResult _outhit)) (.ImpactPoint (Collision|BreakHitResult _outhit)))
      (Effects|SpawnEmitteratLocation "/Game/MeleeSystemPro/Melee_Class/Particles/P_Blood.P_Blood" (.Location (Collision|BreakHitResult _outhit)) :!label _label)
      (Utilities|Struct|SetmembersinS_Weapon_Settings _weaponsettings (- _current_state _decrease_durability) :!label _label_2)
      (else
        (Utilities|IsValid (Actor|GetComponentbyClass (.HitActor (Collision|BreakHitResult _outhit)) "/Game/MeleeSystemPro/BP_Receive_Attack.BP_Receive_Attack_C")
          (:Is%20Valid
            (Class|BPTakeDamage|ITakeDamage(Message) (Actor|GetComponentbyClass (.HitActor (Collision|BreakHitResult _outhit)) "/Game/MeleeSystemPro/BP_Receive_Attack.BP_Receive_Attack_C") (.HitBoneName (Collision|BreakHitResult _outhit)) _returnvalue_4 _character (.Location (Collision|BreakHitResult _outhit)) (.ImpactPoint (Collision|BreakHitResult _outhit)))
            (goto _label))
          (:Is%20Not%20Valid
            (if (!= (.HitActor (Collision|BreakHitResult _outhit)) (Variables|Character|GetCharacter))
              (goto _label_2))))))))

(event Custom|StartFire
  (bind _weaponequipunequip (Variables|Default|GetWeaponEquipUnequip))
  (bind _currentweapon (Variables|/Game/MeleeSystemPro/BP_MeleeWeapon_Equip_Unequip.BP_MeleeWeapon_Equip_Unequip_C|GetCurrentWeapon _weaponequipunequip))
  (bind _weaponsettings (Variables|BP_Weapon_C|GetWeaponSettings _currentweapon))
  (bind (_current_state _attack_animation _start_next_attack _limit_next_attack _speed_attack _attack_reaction_time) (Utilities|Struct|BreakS_Weapon_Settings _weaponsettings))
  (bind _returnvalue (Utilities|Array|Length _attack_animation))
  (bind _returnvalue_2 (<= _current_state 0))
  ;[1 1 1] Fire
  (Utilities|FlowControl|Sequence
    (:then_0
      (goto _label Open))
    (:then_1
      (Utilities|FlowControl|Gate true :!label _label
        (:Exit
          (Utilities|IsValid _weaponequipunequip
            (:Is%20Valid
              (if (Variables|/Game/MeleeSystemPro/BP_MeleeWeapon_Equip_Unequip.BP_MeleeWeapon_Equip_Unequip_C|GetisSwap? _weaponequipunequip)
                (goto _label Close)
                (elif (Variables|/Game/MeleeSystemPro/BP_MeleeWeapon_Equip_Unequip.BP_MeleeWeapon_Equip_Unequip_C|GetisEquiped? _weaponequipunequip)
                  (if _returnvalue_2
                    (goto _label Close)
                    (else
                      (Utilities|FlowControl|Sequence
                        (:then_0
                          (if (Variables|Don'tchange|GetisStop?)
                            (Utilities|FlowControl|RetriggerableDelay (Utilities|Array|Get(acopy) _attack_reaction_time (Variables|Don'tchange|GetComboCounter)))
                            (else
                              (Utilities|FlowControl|RetriggerableDelay (Utilities|Array|Get(acopy) _attack_reaction_time))))
                          (CallFunction|OpenAttack)
                          (CallFunction|Restart)
                          (goto _label))
                        (:then_1
                          (if _returnvalue_2
                            (Development|PrintString "The Weapon Break")
                            (Variables|Don'tchange|SetcanFire? false)
                            (Variables|Don'tchange|SetinCombo? false)
                            (elif (> _returnvalue 1)
                              (if (> (Variables|Don'tchange|GetComboCounter) 0)
                                (if (and (>= (Variables|Don'tchange|GetTimeAttack) (Utilities|Array|Get(acopy) _start_next_attack (- (Variables|Don'tchange|GetComboCounter) 1))) (<= (Variables|Don'tchange|GetTimeAttack) (Utilities|Array|Get(acopy) _limit_next_attack (- (Variables|Don'tchange|GetComboCounter) 1))))
                                  (switch int (Variables|Don'tchange|GetComboCounter) :!label _label_2
                                    (:Default
                                      (CallFunction|EnableHit)
                                      (Animation|Montage|MontagePlay (Components|SkeletalMesh|GetAnimInstance (Variables|/Script/Engine.Character|GetMesh (Variables|Character|GetCharacter))) (Utilities|Array|Get(acopy) _attack_animation (Variables|Don'tchange|GetComboCounter)) (Utilities|Array|Get(acopy) _speed_attack (Variables|Don'tchange|GetComboCounter)) "MontageLength" 0.0 true)
                                      (Utilities|FlowControl|Sequence
                                        (:then_0
                                          (Utilities|FlowControl|Delay (Utilities|Array|Get(acopy) _attack_reaction_time (Variables|Don'tchange|GetComboCounter)))
                                          (CallFunction|DisableHit))
                                        (:then_1
                                          (Variables|Don'tchange|SetinCombo? true)
                                          (if (== (Variables|Don'tchange|GetComboCounter) (- _returnvalue 1))
                                            (Variables|Don'tchange|SetComboCounter 0)
                                            (Utilities|FlowControl|Delay (Utilities|Array|Get(acopy) _attack_reaction_time (Variables|Don'tchange|GetComboCounter)))
                                            (Variables|Don'tchange|SetinCombo? false)
                                            (else
                                              (Variables|Don'tchange|SetComboCounter (+ (Variables|Don'tchange|GetComboCounter) 1))
                                              (Variables|Don'tchange|SetinCombo? false)))
                                          (Variables|Don'tchange|SetcanFire? false)))))
                                  (elif (> (Variables|Don'tchange|GetTimeAttack) (Utilities|Array|Get(acopy) _limit_next_attack (- (Variables|Don'tchange|GetComboCounter) 1)))
                                    (Variables|Don'tchange|SetTimeAttack 0.0)
                                    (Variables|Don'tchange|SetComboCounter 0)
                                    (Variables|Don'tchange|SetinCombo? false)
                                    (goto _label_2)))
                                (elif (not (Variables|Don'tchange|GetinCombo?))
                                  (goto _label_2)))
                              (else
                                (Utilities|FlowControl|Gate false
                                  (:Exit
                                    (Variables|Don'tchange|SetinCombo? true)
                                    (CallFunction|CloseAttack)
                                    (CallFunction|EnableHit)
                                    (Animation|Montage|MontagePlay (Components|SkeletalMesh|GetAnimInstance (Variables|/Script/Engine.Character|GetMesh (Variables|Character|GetCharacter))) (Utilities|Array|Get(acopy) _attack_animation (Variables|Don'tchange|GetComboCounter)) (Utilities|Array|Get(acopy) _speed_attack (Variables|Don'tchange|GetComboCounter)) "MontageLength" 0.0 true)
                                    (Utilities|FlowControl|Sequence
                                      (:then_0
                                        (Utilities|FlowControl|Delay (Utilities|Array|Get(acopy) _attack_reaction_time (Variables|Don'tchange|GetComboCounter)))
                                        (CallFunction|DisableHit))
                                      (:then_1
                                        (Variables|Don'tchange|SetinCombo? false)
                                        (Variables|Don'tchange|SetcanFire? false))))))))))))
                  (else
                    (goto _label Close)))))
            (:Is%20Not%20Valid
              (goto _label Close))))))))

(event Custom|StopFire
  (bind _weaponequipunequip (Variables|Default|GetWeaponEquipUnequip))
  (bind _currentweapon (Variables|/Game/MeleeSystemPro/BP_MeleeWeapon_Equip_Unequip.BP_MeleeWeapon_Equip_Unequip_C|GetCurrentWeapon _weaponequipunequip))
  (bind _weaponsettings (Variables|BP_Weapon_C|GetWeaponSettings _currentweapon))
  (bind (_current_state _attack_animation _start_next_attack _limit_next_attack _speed_attack _attack_reaction_time) (Utilities|Struct|BreakS_Weapon_Settings _weaponsettings))
  (bind _returnvalue (Utilities|Array|Length _attack_animation))
  (bind _returnvalue_2 (<= _current_state 0))
  ;[1 1 1] Fire
  (Utilities|FlowControl|Gate true) ; enters at Close
)

(event Custom|Restart
  ;[1 1 1] Fire
  (bind _returnvalue (Utilities|Time|SetTimerbyEvent (delegate Custom|Updating) 0.01 true)))

(event Custom|FireRelease
  (params (WeaponEquipUnequip :type BP%20Melee%20Weapon%20Equip%20Unequip%20Object%20Reference))
  ;[1 1 1] Fire
  (Variables|Default|SetWeaponEquipUnequip WeaponEquipUnequip)
  (CallFunction|StopFire)
  (Variables|Don'tchange|SetisStop? true)
  (Utilities|FlowControl|Delay 0.2))

(event Custom|OpenAttack
  (bind _weaponequipunequip (Variables|Default|GetWeaponEquipUnequip))
  (bind _combocounter (Variables|Don'tchange|GetComboCounter))
  (bind _currentweapon (Variables|/Game/MeleeSystemPro/BP_MeleeWeapon_Equip_Unequip.BP_MeleeWeapon_Equip_Unequip_C|GetCurrentWeapon _weaponequipunequip))
  (bind _weaponsettings (Variables|BP_Weapon_C|GetWeaponSettings _currentweapon))
  (bind (_current_state _attack_animation _start_next_attack _limit_next_attack _speed_attack _attack_reaction_time) (Utilities|Struct|BreakS_Weapon_Settings _weaponsettings))
  ;[1 1 1] Fire
  (Utilities|FlowControl|Gate false) ; enters at Open
)

(event Custom|CloseAttack
  (bind _weaponequipunequip (Variables|Default|GetWeaponEquipUnequip))
  (bind _combocounter (Variables|Don'tchange|GetComboCounter))
  (bind _currentweapon (Variables|/Game/MeleeSystemPro/BP_MeleeWeapon_Equip_Unequip.BP_MeleeWeapon_Equip_Unequip_C|GetCurrentWeapon _weaponequipunequip))
  (bind _weaponsettings (Variables|BP_Weapon_C|GetWeaponSettings _currentweapon))
  (bind (_current_state _attack_animation _start_next_attack _limit_next_attack _speed_attack _attack_reaction_time) (Utilities|Struct|BreakS_Weapon_Settings _weaponsettings))
  ;[1 1 1] Fire
  (Utilities|FlowControl|Gate false) ; enters at Close
)

(event Custom|DisableHit
  ;[1 1 1] Hit
  (Collision|SetCollisionEnabled (Variables|Default|GetCapsuleHit) "NoCollision")
  (Utilities|Time|ClearandInvalidateTimerbyHandle (stale OnComponentBeginOverlap(CapsuleHit) _returnvalue)))

(event Custom|Updating
  (bind _weaponequipunequip (Variables|Default|GetWeaponEquipUnequip))
  (bind _currentweapon (Variables|/Game/MeleeSystemPro/BP_MeleeWeapon_Equip_Unequip.BP_MeleeWeapon_Equip_Unequip_C|GetCurrentWeapon _weaponequipunequip))
  (bind _weaponsettings (Variables|BP_Weapon_C|GetWeaponSettings _currentweapon))
  (bind (_current_state _attack_animation _start_next_attack _limit_next_attack _speed_attack _attack_reaction_time) (Utilities|Struct|BreakS_Weapon_Settings _weaponsettings))
  ;[1 1 1] Fire
  (if (> (Utilities|Array|Length _attack_animation) 1)
    (Variables|Don'tchange|SetCurrentWeapoon (- (Variables|Don'tchange|GetComboCounter) 1))
    (else
      (Variables|Don'tchange|SetCurrentWeapoon 0)))
  (Variables|Don'tchange|SetTimeAttack (+ (Variables|Don'tchange|GetTimeAttack) 0.01))
  (if (>= (Variables|Don'tchange|GetTimeAttack) (Utilities|Array|Get(acopy) _attack_reaction_time (Variables|Don'tchange|GetCurrentWeapoon)))
    (Utilities|Time|ClearandInvalidateTimerbyHandle (stale Custom|FirePress _returnvalue))
    (CallFunction|OpenAttack)
    (Variables|Don'tchange|SetTimeAttack 0.0)
    (Variables|Don'tchange|SetComboCounter 0)
    (Variables|Don'tchange|SetcanFire? false)))

(event EventBeginPlay
  ;[1 1 1] Begin
  (Variables|Character|SetCharacter (Game|GetPlayerCharacter 0))
  (Rendering|SetVisibility (Variables|Default|GetWidget) false false)
  (bind _returnvalue (UserInterface|CreateWidget "/Game/MeleeSystemPro/Melee_Class/Widget/W_Weapon_Widget.W_Weapon_Widget_C"))
  (Variables|Don'tchange|SetWidgetWeapon _returnvalue))

(event EventInteractionChar
  (params (Weapon_Equip_Unequip :type BP%20Melee%20Weapon%20Equip%20Unequip%20Object%20Reference))
  ;[1 1 1] Pickup Item
  (bind _output_get (Variables|Default|SetWeaponEquipUnequip Weapon_Equip_Unequip))
  (Default|PItem _output_get self (Variables|Don'tchange|GetCurrentState)))

(fn ConstructionScript
  (Variables|Weapon|SetWeaponSettings (Utilities|Struct|MakeS_Weapon_Settings (.weapon_type (Variables|Weapon|GetWeaponSettings)) (.weapon_class (Variables|Weapon|GetWeaponSettings)) (.decrease_durability (Variables|Weapon|GetWeaponSettings)) (.current_state (Variables|Weapon|GetWeaponSettings)) (.damage (Variables|Weapon|GetWeaponSettings)) (.weapon_image (Variables|Weapon|GetWeaponSettings)) (.pickup_animation (Variables|Weapon|GetWeaponSettings)) (.replaceif (Variables|Weapon|GetWeaponSettings)) (.sound_pickup (Variables|Weapon|GetWeaponSettings)) (.speed_pickup (Variables|Weapon|GetWeaponSettings)) (.equip_animation (Variables|Weapon|GetWeaponSettings)) (.unequip_animation (Variables|Weapon|GetWeaponSettings)) (.sound_equip (Variables|Weapon|GetWeaponSettings)) (.sound_unequip (Variables|Weapon|GetWeaponSettings)) (.speed_equip (Variables|Weapon|GetWeaponSettings)) (.speed_unequip (Variables|Weapon|GetWeaponSettings)) (.equip_socket_name (Variables|Weapon|GetWeaponSettings)) (.attach_time_equip (Variables|Weapon|GetWeaponSettings)) (.unequip_socket_name (Variables|Weapon|GetWeaponSettings)) (.attach_time_unequip (Variables|Weapon|GetWeaponSettings)) (.attack_animation (Variables|Weapon|GetWeaponSettings)) (.start_next_attack (Variables|Weapon|GetWeaponSettings)) (.limit_next_attack (Variables|Weapon|GetWeaponSettings)) (.sound_hit (Variables|Weapon|GetWeaponSettings)) (.speed_attack (Variables|Weapon|GetWeaponSettings)) (.attack_reaction_time (Variables|Weapon|GetWeaponSettings)) (.particle_socket_name (Variables|Weapon|GetWeaponSettings)) (.particle_emitter (Variables|Weapon|GetWeaponSettings)) (.sound_missed_attack (Variables|Weapon|GetWeaponSettings)))))