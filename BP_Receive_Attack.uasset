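; BP_Receive_Attack gives an enemy Character health, a health-bar widget, hit reactions and death handling.
; BeginReceiveAttack binds the HUD, Tick sets its bar from health over a hardcoded 100, and ITakeDamage routes to Hit or GoRagdoll.
; Hit briefly blends impulse-driven physics from the struck bone, then switches the mesh to single-node animation.
; GoRagdoll plays the death animation, or ragdolls without one, then destroys the Character after a delay.
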(event Custom|BeginReceiveAttack
  (params (Widget :type Widget%20Component%20Object%20Reference) (Character :type Character%20Object%20Reference))
  ;[1 1 1] Begin
  (Variables|Character|SetCharacter Character)
  (Variables|Don'tchange|SetWidget Widget)
  (Variables|Health|SetCurrentHealth (Variables|Health|GetMaxHealth))
  (bind _returnvalue (UserInterface|CreateWidget "/Game/MeleeSystemPro/Melee_Class/Widget/W_Enemy_HUD.W_Enemy_HUD_C" 0 self))
  (bind _output_get (Variables|Don'tchange|SetHUDEnemy _returnvalue))
  (UserInterface|SetWidget (Variables|Don'tchange|GetWidget) _output_get)
  (Rendering|SetVisibility (Variables|Don'tchange|GetWidget) (Variables|Widget|GetisWidgetVisible?) false))

(event Custom|GoRagdoll
  (params (Impulse :type Vector) (BoneName :type Name))
  (bind _death_animmontage (Variables|Character|GetDeath_AnimMontage))
  (bind _character (Variables|Character|GetCharacter))
  (bind _bone__pelvis_or_hips_ (Variables|Character|GetBone%20%28Pelvis%20or%20Hips%29))
  (bind _returnvalue (Utilities|Name|MakeLiteralName _bone__pelvis_or_hips_))
  (bind _mesh (Variables|/Script/Engine.Character|GetMesh _character))
  (Components|Animation|PlayAnimation (Variables|/Script/Engine.Character|GetMesh _character) _death_animmontage false)
  (if (Utilities|IsValid _death_animmontage)
    _
    (else
      (Class|PrimitiveComponent|SetMassOverrideinKg _mesh "None" 1.8e+02 true)
      (Class|SkeletalMeshComponent|SetAllBodiesBelowSimulatePhysics _mesh _returnvalue true true)
      (Physics|AddImpulse _mesh Impulse BoneName false)
      (Class|SkeletalMeshComponent|SetAllBodiesBelowPhysicsBlendWeight _mesh _returnvalue 1.0 false true)))
  (Pawn|Components|CharacterMovement|SetMovementMode (Variables|/Script/Engine.Character|GetCharacterMovement _character) "MOVE_None" 0)
  (Collision|SetCollisionEnabled (Variables|/Script/Engine.Character|GetCapsuleComponent (Variables|Character|GetCharacter)) "NoCollision")
  (Utilities|FlowControl|Delay (Variables|Health|GetDestroyActorTime))
  (Actor|DestroyActor _character))

(event Custom|Hit
  (bind _character (Variables|Character|GetCharacter))
  (bind _bonehit (Variables|Don'tChange|GetBoneHit))
  (bind _character_2 (Variables|Character|GetCharacter))
  (bind _mesh (Variables|/Script/Engine.Character|GetMesh _character_2))
  (bind _mesh_2 (Variables|/Script/Engine.Character|GetMesh _character))
  (Components|Movement|StopMovementImmediately (Variables|/Script/Engine.Character|GetCharacterMovement _character_2))
  (Class|SkeletalMeshComponent|SetAllBodiesBelowSimulatePhysics _mesh _bonehit true true)
  (Physics|AddImpulseatLocation (Variables|/Script/Engine.Character|GetMesh (Variables|Character|GetCharacter)) (Variables|Don'tChange|GetHitImpulse) (Variables|Don'tChange|GetHitLoc) _bonehit)
  (Class|SkeletalMeshComponent|SetAllBodiesPhysicsBlendWeight _mesh 0.3 false)
  (Utilities|FlowControl|Delay 1.0)
  (if (not (Variables|Don'tChange|GetisDead?))
    (Physics|SetSimulatePhysics _mesh_2 false)
    (Components|Animation|SetAnimationMode _mesh_2 "AnimationSingleNode")))

(event EventTick
  (params (DeltaSeconds :type Float%20%28single-precision%29))
  (Progress|SetPercent (Variables|/Game/MeleeSystemPro/Melee_Class/Widget/W_Enemy_HUD.W_Enemy_HUD_C|GetProgressBar_92 (Variables|Don'tchange|GetHUDEnemy)) (/ (Variables|Health|GetCurrentHealth) 1e+02)))

(event EventITakeDamage
  (params (BoneName :type Name :default "None") (Damage :type Float%20%28single-precision%29) (Sender :type Actor%20Object%20Reference) (HitLocation :type Vector :default "0, 0, 0") (HitBommLocation :type Vector :default "0, 0, 0"))
  (Variables|Don'tChange|SetBoneHit BoneName)
  (Variables|Don'tChange|SetPlayer Sender)
  (Variables|Don'tChange|SetHitLoc HitLocation)
  (Variables|Don'tChange|SetHitImpulse HitBommLocation)
  (bind _output_get (Variables|Health|SetCurrentHealth (- (Variables|Health|GetCurrentHealth) Damage)))
  (bind _output_get_2 (Variables|Don'tChange|SetisDead? (<= _output_get 0.0)))
  (if _output_get_2
    (CallFunction|GoRagdoll (Variables|Don'tChange|GetHitImpulse) (Variables|Don'tChange|GetBoneHit))
    (else
      (CallFunction|Hit))))